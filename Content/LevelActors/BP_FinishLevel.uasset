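; BP_FinishLevel is a level-end trigger actor that sends the player to the next map.
; When an actor implementing BPI_MainCharacter overlaps the Detection box, it fires once, disabling input and showing a W_FadeOut widget.
; After a short delay it opens the level named by NextLevel.
; The construction script sizes the box from DetectionExtents.
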(event `self.Detection.OnComponentBeginOverlap`
  (params (OverlappedComponent :type "PrimitiveComponent Object Reference") (OtherActor :type "Actor Object Reference") (OtherComp :type "PrimitiveComponent Object Reference") (OtherBodyIndex :type Integer) (bFromSweep :type Boolean) (SweepResult :type "HitResult Structure (by ref)"))
  (if (`KismetSystemLibrary.DoesImplementInterface` OtherActor "/Game/MainCharacter/BPI_MainCharacter.BPI_MainCharacter_C")
    (`/Engine/EditorBlueprintResources/StandardMacros.DoOnce` false
      (:`Completed`
        (`self.DisableInput` OtherActor (`GameplayStatics.GetPlayerController` 0))
        (bind _returnvalue (`|CreateWidget` "/Game/Widgets/W_FadeOut.W_FadeOut_C"))
        (`UserWidget.AddToViewport` _returnvalue 0)
        (`KismetSystemLibrary.Delay` 0.5)
        (`GameplayStatics.OpenLevel` (`self.NextLevel`))))))

(fn `UserConstructionScript`
  (`BoxComponent.SetBoxExtent` (`self.Detection`) (`self.DetectionExtents`) true))