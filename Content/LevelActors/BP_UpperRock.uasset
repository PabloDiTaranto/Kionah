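; BP_UpperRock is a level actor rock that rises and lowers between two marker components, Init and End.
; GoUp plays a timeline that lerps the mesh's world location from Init to End, and GoDown reverses it.
; Two helper events set up the endpoints: one copies the mesh's current location to End, the other snaps the mesh back to Init.
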(event `GoUp`
  (bind (_direction _alphamove) (`Timeline|GoUpTimeline` :!label _label)
    (:`Update`
      (`SceneComponent.K2_SetWorldLocation` (`self.StaticMesh`) (`KismetMathLibrary.VLerp` (`SceneComponent.K2_GetComponentLocation` (`self.Init`)) (`SceneComponent.K2_GetComponentLocation` (`self.End`)) _alphamove) false false))))

(event `GoDown`
  (goto _label :!via `Reverse`))

(event `SetEndLocaticon`
  (`SceneComponent.K2_SetWorldLocation` (`self.End`) (`SceneComponent.K2_GetComponentLocation` (`self.StaticMesh`)) false false))

(event `AlignToInit`
  (`SceneComponent.K2_SetWorldLocation` (`self.StaticMesh`) (`SceneComponent.K2_GetComponentLocation` (`self.Init`)) false false))

(fn `UserConstructionScript`)