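; BP_Hushtail is the Blueprint for the Hushtail pawn, exposing events to move or place it in the level.
; MoveTo sends it to a target actor with AIMoveTo, then on success uses a timeline to lerp its rotation along the shortest path to match the target's.
; TranslateTo sets its transform directly, without sweep or teleport physics.
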(event `self.ReceiveTick`
  (params (DeltaSeconds :type "Float (single-precision)")))

(event `MoveTo`
  (params (TargetActor :type "Actor Object Reference"))
  (bind (_returnvalue_location _returnvalue_rotation) (`KismetMathLibrary.BreakTransform` (`self.GetTransform` TargetActor)))
  (`|AIMoveTo` self (0.0 0.0 0.0) TargetActor
    (:`OnSuccess`
      (set `self.OriginRot` (`self.K2_GetActorRotation`))
      (set `self.FinalRot` _returnvalue_rotation)
      (bind (_direction _newtrack_0) (`Timeline|RotateTimeline`)
        (:`Update`
          (`self.K2_SetActorRotation` (`KismetMathLibrary.RLerp` (`self.OriginRot`) (`self.FinalRot`) _newtrack_0 true)))))))

(event `TranslateTo`
  (params (NewTransform :type "Transform Structure (by ref)"))
  (`self.K2_SetActorTransform` NewTransform))

(fn `UserConstructionScript`)