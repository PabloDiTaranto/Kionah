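; BP_RespawnByFall is a level trigger that respawns the main character on entering it, as after a fall.
; Overlap with the Detection box checks for BPI_MainCharacter and sends RespawnByFallMessage with the RespawnPoint's world transform.
; A DoOnce gate, reset after a short delay, blocks repeated triggers.
; The construction script sizes the box from CollisionExtents.
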(event `self.Detection.OnComponentBeginOverlap`
  (params (OverlappedComponent :type "PrimitiveComponent Object Reference") (OtherActor :type "Actor Object Reference") (OtherComp :type "PrimitiveComponent Object Reference") (OtherBodyIndex :type Integer) (bFromSweep :type Boolean) (SweepResult :type "HitResult Structure (by ref)"))
  (if (`KismetSystemLibrary.DoesImplementInterface` OtherActor "/Game/MainCharacter/BPI_MainCharacter.BPI_MainCharacter_C")
    (`/Engine/EditorBlueprintResources/StandardMacros.DoOnce` false :!label _label
      (:`Completed`
        (message `/Game/MainCharacter/BPI_MainCharacter.RespawnByFall` OtherActor (`SceneComponent.K2_GetComponentToWorld` (`self.RespawnPoint`)))
        (`KismetSystemLibrary.Delay` 0.2)
        (`self.ResetDoOnce`)))))

(event `ResetDoOnce`
  (goto _label :!via `Reset`))

(fn `UserConstructionScript`
  (`BoxComponent.SetBoxExtent` (`self.Detection`) (`self.CollisionExtents`) true))