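; BP_MovableRock is a level actor rock that the main character can physically move only while in one specific size state.
; When an actor implementing BPI_MainCharacter enters the DetectPlayer component, it queries that actor's size and switches mesh physics simulation on for that size, off otherwise.
; The starting transform is cached on BeginPlay, and a Respawn event sets the actor transform back to it.
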(event `self.ReceiveBeginPlay`
  (set `self.Origin` (`self.GetTransform`)))

(event `self.Detect Player.OnComponentBeginOverlap`
  (params (OverlappedComponent :type "PrimitiveComponent Object Reference") (OtherActor :type "Actor Object Reference") (OtherComp :type "PrimitiveComponent Object Reference") (OtherBodyIndex :type Integer) (bFromSweep :type Boolean) (SweepResult :type "HitResult Structure (by ref)"))
  (bind _staticmesh (`self.StaticMesh`))
  (if (`KismetSystemLibrary.DoesImplementInterface` OtherActor "/Game/MainCharacter/BPI_MainCharacter.BPI_MainCharacter_C")
    (bind _size (message `/Game/MainCharacter/BPI_MainCharacter.RequestSize` OtherActor))
    (if (`|EnumInequality` _size "NewEnumerator2")
      (`PrimitiveComponent.SetSimulatePhysics` _staticmesh false)
      (else
        (`PrimitiveComponent.SetSimulatePhysics` _staticmesh true)))))

(event `/Game/Interfaces/BPI_MovableRocks.Respawn`
  (`self.K2_SetActorTransform` (`self.Origin`)))

(fn `UserConstructionScript`)