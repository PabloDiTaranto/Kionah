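; BP_DescendingPlatform is a level platform that descends when the main character enters its DetectPlayer volume at one specific size.
; The size is queried through BPI_MainCharacter, and a match plays a timeline lerping the mesh between the IntialPos and FinalPos components.
; Leaving the volume, or entering at another size (which also prints a debug string), reverses the timeline after a fixed delay.
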(event `self.DetectPlayer.OnComponentBeginOverlap`
  (params (OverlappedComponent :type "PrimitiveComponent Object Reference") (OtherActor :type "Actor Object Reference") (OtherComp :type "PrimitiveComponent Object Reference") (OtherBodyIndex :type Integer) (bFromSweep :type Boolean) (SweepResult :type "HitResult Structure (by ref)"))
  (if (`KismetSystemLibrary.DoesImplementInterface` OtherActor "/Game/MainCharacter/BPI_MainCharacter.BPI_MainCharacter_C")
    (bind _size (message `/Game/MainCharacter/BPI_MainCharacter.RequestSize` OtherActor))
    (if (`|EnumEquality` _size "NewEnumerator2")
      (`self.DownPlatform`)
      (else
        (`self.UpPlatform`)
        (`KismetSystemLibrary.PrintString` "Hello")))))

(event `DownPlatform`
  (bind (_direction _timedown) (`Timeline|MovePlatform` :!label _label)
    (:`Update`
      (`SceneComponent.K2_SetRelativeLocation` (`self.StaticMesh`) (`KismetMathLibrary.VLerp` (`SceneComponent.RelativeLocation` (`self.IntialPos`)) (`SceneComponent.RelativeLocation` (`self.FinalPos`)) _timedown) false false))))

(event `UpPlatform`
  (`KismetSystemLibrary.Delay` 6.0)
  (goto _label :!via `Reverse`))

(event `self.DetectPlayer.OnComponentEndOverlap`
  (params (OverlappedComponent :type "PrimitiveComponent Object Reference") (OtherActor :type "Actor Object Reference") (OtherComp :type "PrimitiveComponent Object Reference") (OtherBodyIndex :type Integer))
  (if (`KismetSystemLibrary.DoesImplementInterface` OtherActor "/Game/MainCharacter/BPI_MainCharacter.BPI_MainCharacter_C")
    (`self.UpPlatform`)))

(fn `UserConstructionScript`)