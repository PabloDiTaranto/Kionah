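; BP_FallingRocks is a level actor that manages a group of BP_FallRock actors and moves them up and down together.
; Spawn and remove events add rocks at the actor's transform or destroy the last one, tracked in RocksSpawned.
; Rocks are attached to the Father component, with BeginPlay re-attaching every listed rock.
; GoUp and GoDown play or reverse a timeline that lerps Father between Init and End locations.
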(event `self.ReceiveBeginPlay`
  (`self.AttachToFather`))

(event `SpawnFallRock`
  (bind _returnvalue (`|SpawnActorFromClass` "/Game/LevelActors/BP_FallRock.BP_FallRock_C" (`self.GetTransform`) "Undefined" "OverrideRootScale" null null))
  (`self.K2_AttachToComponent` _returnvalue (`self.Father`) "None" "KeepWorld" "KeepWorld" "KeepWorld" false)
  (`KismetArrayLibrary.Array_Add` (`self.RocksSpawned`) _returnvalue))

(event `RemoveLastRock`
  (bind _returnvalue (`KismetArrayLibrary.Array_Length` (`self.RocksSpawned`)))
  (bind _returnvalue_2 (- _returnvalue 1))
  (bind _output (`|GetArrayItem` (`self.RocksSpawned`) _returnvalue_2))
  (if (> _returnvalue 0)
    (`self.K2_DetachFromActor` _output "KeepRelative" "KeepRelative" "KeepRelative")
    (`self.K2_DestroyActor` _output)
    (`KismetArrayLibrary.Array_Remove` (`self.RocksSpawned`) _returnvalue_2)))

(event `GoUp`
  (bind (_direction _alphamove) (`Timeline|GoUpTimeline` :!label _label)
    (:`Update`
      (`SceneComponent.K2_SetRelativeLocation` (`self.Father`) (`KismetMathLibrary.VLerp` (`SceneComponent.RelativeLocation` (`self.Init`)) (`SceneComponent.RelativeLocation` (`self.End`)) _alphamove) false false))))

(event `GoDown`
  (goto _label :!via `Reverse`))

(event `AttachToFather`
  (for _array_element (`self.RocksSpawned`)
    (`self.K2_AttachToComponent` _array_element (`self.Father`) "None" "KeepWorld" "KeepWorld" "KeepWorld" false)))

(fn `UserConstructionScript`)